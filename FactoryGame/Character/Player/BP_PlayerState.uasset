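; BP_PlayerState is the player state Blueprint, declaring an interface for player chat, buildable-construction notification and a per-player recipe shopping list.
; Shopping list operations cover add, remove, set count, clear and sort, with Server_ events and an OnRep function pointing to a replicated list.
; Every event and function here is an empty stub or returns a default, so the file holds signatures without working logic.
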(event `BroadcastChatMessage`
  (params (ChatMessageIn :type Text)))

(event `ReceiveChatMessage`
  (params (ChatMessageIn :type Text) (ChatSender :type Text)))

(event `OnBuildableConstructed`
  (params (itemDescriptor :type "FGItemDescriptor Class Reference")))

(event `Server_AddRecipeToShoppingList`
  (params (recipe :type "FGRecipe Class Reference") (NumRecipes :type Integer)))

(event `Server_SetNumRecipesInShoppingList`
  (params (recipe :type "FGRecipe Class Reference") (NumRecipes :type Integer)))

(event `Server_RemoveRecupeFromShoppingList`
  (params (recipe :type "FGRecipe Class Reference") (NumRecipes :type Integer)))

(event `Server_ClearShoppingList`)

(fn `AddRecipeToShoppingList`
  (params (recipe :type "FGRecipe Class Reference") (NumRecipes :type Integer)))

(fn `AddToShoppingList`
  (params (recipe :type "FGRecipe Class Reference") (Amount :type Integer))
  (returns (Success :type Boolean))
  (return false))

(fn `ClearShoppingData`
  (returns (Succes :type Boolean))
  (return false))

(fn `ClearShoppingList`)

(fn `GetShippingListData`
  (returns (ShippingList :type "Array of /Game/FactoryGame/Interface/UI/InGame/RecipeAmountStruct Structure"))
  (return))

(fn `GetShoppingListSortIndex`
  (params (RecipeAmountStruct :type "/Game/FactoryGame/Interface/UI/InGame/RecipeAmountStruct Structure (by ref)"))
  (returns (ReturnValue :type Integer))
  (return 0))

(fn `OnRep_mShoppingList`)

(fn `PonderUpdatingShoppingList`
  (params (InputPin :type "FGItemDescriptor Class Reference")))

(fn `RemoveFromShoppingList`
  (params (recipe :type "FGRecipe Class Reference") (Amount :type Integer))
  (returns (Success :type Boolean))
  (return false))

(fn `RemoveRecipeFromShoppingList`
  (params (recipe :type "FGRecipe Class Reference") (NumRecipes :type Integer)))

(fn `SetNumInShoppingList`
  (params (recipe :type "FGRecipe Class Reference") (Amount :type Integer))
  (returns (Success :type Boolean))
  (return false))

(fn `SetNumRecipeInShoppingList`
  (params (recipe :type "FGRecipe Class Reference") (NumRecipes :type Integer)))

(fn `ShoppingListUpdated`)

(fn `SortShoppingList`)

(fn `UserConstructionScript`)