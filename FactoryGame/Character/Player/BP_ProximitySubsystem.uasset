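; Player proximity subsystem Blueprint whose function names describe ambient wildlife VFX and SFX driven by nearby foliage, map area, ecosystem density and quality settings.
; Nearly every function here is an empty stub or returns zero or false, so none of that spawning, timer or density logic is implemented.
; Only BeginPlay, Tick, map-area entry and pawn-change events do anything, each simply forwarding to the parent class.
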(event `self.ReceiveBeginPlay`
  (`parent.ReceiveBeginPlay`))

(event `self.ReceiveTick`
  (params (DeltaSeconds :type "Float (single-precision)"))
  (`parent.ReceiveTick` DeltaSeconds))

(event `EnterAreaTimer`)

(event `self.OnEnteredMapArea`
  (params (playerController :type "FGPlayerControllerBase Object Reference") (newArea :type "FGMapArea Class Reference"))
  (`parent.OnEnteredMapArea` playerController newArea))

(event `Spawn_AmbientLife_Far`)

(event `Spawn_AmbientLife_Near`)

(event `Spawn_FallingLeaves`)

(event `self.OnPawnChanged`
  (params (newPawn :type "Pawn Object Reference"))
  (`parent.OnPawnChanged` newPawn))

(fn `CalculateEcoSystemByInt`
  (params (Bushes :type Integer) (Trees :type Integer) (Rocks :type Integer) (Flowers :type Integer) (TotalAmount :type Integer))
  (returns (TypeOfEcoSystem :type Integer))
  (return 0))

(fn `CheckAreaAmbience`)

(fn `CheckAreaDensity`
  (params (AreaRadius :type "Float (double-precision)") (`%ModBy` :type Integer))
  (returns (CalculatedAmount :type Integer))
  (return 0))

(fn `CheckAreaDensityByType`
  (params (AreaRadius :type "Float (double-precision)") (`%ModBy` :type Integer))
  (returns (`%ModBushes` :type Integer) (`%ModTrees` :type Integer) (`%ModRocks` :type Integer) (`%ModFlowers` :type Integer) (TotalAmount :type Integer))
  (return 0 0 0 0 0))

(fn `CheckAreaDynamicDensity`
  (params (AreaRadius :type "Float (double-precision)"))
  (returns (AmountOfBushes :type Integer) (AmountOfTrees :type Integer) (AmountOfRocks :type Integer) (AmountOfFlowers :type Integer) (TotalAmount :type Integer))
  (return 0 0 0 0 0))

(fn `CheckContainedCachedInstances`
  (params (MaxAmbienceInstances :type Integer)))

(fn `CheckContainedSFXCachedInstances`
  (params (MaxSFXInstances :type Integer)))

(fn `CheckSFXDynamicAreaAmbience`)

(fn `CheckSingleLocationAmbience`)

(fn `CheckSingleLocationSFX`)

(fn `DuneDesert_AmbientLife_VFX`)

(fn `ForecastPredictionOnAreas`)

(fn `GetFoliageID`
  (params (FoliageIDs :type "Array of Integer (by ref)"))
  (returns (ChosenFoliageID :type Integer) (GetFoliageIndex :type Integer))
  (return 0 0))

(fn `GetValueByQuality`
  (params (Low :type "Float (double-precision)") (Medium :type "Float (double-precision)") (High :type "Float (double-precision)") (Ultra :type "Float (double-precision)") (UltraPlus :type "Float (double-precision)"))
  (returns (ReturnValue :type "Float (double-precision)"))
  (return 0.0))

(fn `IsFoliageInSight`
  (params (FoliageLocation :type "Vector Structure"))
  (returns (IsFoliageInSight :type Boolean))
  (return false))

(fn `IsFoliageNear`
  (params (FoliageLocation :type "Vector Structure") (SetDistanceForNearRadius :type "Float (double-precision)"))
  (returns (isNear :type Boolean))
  (return false))

(fn `IsFoliageWithinAttenuation`
  (params (`Ak Event` :type "AkAudioEvent Object Reference") (FoliageLocation :type "Vector Structure"))
  (returns (IsWithinRadius :type Boolean))
  (return false))

(fn `OnEnteredNewArea`)

(fn `RandomBackwardDirectionalVector`
  (returns (FoliageRemovalSystem :type "FGFoliageRemovalSubsystem Object Reference") (RandomDirectionalBackwardVector :type "Vector Structure"))
  (return null (0.0 0.0 0.0)))

(fn `RandomForwardDirectionalVector`
  (returns (FoliageRemovalSystem :type "FGFoliageRemovalSubsystem Object Reference") (RandomDirectionalForwardVector :type "Vector Structure"))
  (return null (0.0 0.0 0.0)))

(fn `RemoveContainedFoliageIndex`
  (params (LifeArray :type "Array of Integer (by ref)") (ContainedLifeID :type Integer)))

(fn `RemoveContainedSFXIndex`
  (params (SFXArray :type "Array of Integer (by ref)") (ContainedLifeID :type Integer)))

(fn `SetEcoSystemByArea`
  (params (TypeOfEcoSystemInt :type Integer)))

(fn `SetupAreaAmbienceByFoliageType`
  (params (MeshIDs :type "Array of Integer (by ref)") (FoliageType :type "EProximityEffectTypes Enum" :default "PET_None") (InstancedStaticMeshComp :type "InstancedStaticMeshComponent Object Reference") (FoliageLocation :type "Vector Structure") (InstanceId :type Integer)))

(fn `SetupAreaSFXFoliageType`
  (params (MeshIndex :type "Array of Integer (by ref)") (FoliageType :type "EProximityEffectTypes Enum" :default "PET_None") (StaticMeshCompReference :type "InstancedStaticMeshComponent Object Reference") (IstanceID :type Integer) (FoliageLocation :type "Vector Structure")))

(fn `SetupMapAreaEffect`
  (params (NewArea :type "FGMapArea Class Reference")))

(fn `SetupQuality`)

(fn `SetupSingleAmbienceByFoliageType`
  (params (MeshIDs :type "Array of Integer (by ref)") (FoliageType :type "EProximityEffectTypes Enum" :default "PET_None") (InstancedStaticMeshComp :type "InstancedStaticMeshComponent Object Reference") (FoliageLocation :type "Vector Structure") (InstanceId :type Integer)))

(fn `SetupSingleSFXFoliageType`
  (params (MeshIndex :type "Array of Integer (by ref)") (FoliageType :type "EProximityEffectTypes Enum" :default "PET_None") (StaticMeshCompReference :type "InstancedStaticMeshComponent Object Reference") (FoliageLocation :type "Vector Structure") (InstanceId :type Integer)))

(fn `SFXSwitchOnEnteredArea`)

(fn `Spawn_Beetles_01_VFX`)

(fn `Spawn_Butterflies_VFX`)

(fn `Spawn_Falling_VFX`
  (params (FoliageRemovalSystem :type "FGFoliageRemovalSubsystem Object Reference")))

(fn `Spawn_FarVFX`)

(fn `Spawn_FireFlies_VFX`)

(fn `Spawn_Flies_VFX`)

(fn `Spawn_Ground_Scatter_VFX`
  (params (IsInCave :type Boolean)))

(fn `Spawn_NearVFX`
  (params (FoliageRemovalSystem :type "FGFoliageRemovalSubsystem Object Reference")))

(fn `Spawn_Scatter_Flying_VFX`
  (params (TreeLocation :type "Vector Structure") (bIsInCave :type Boolean)))

(fn `SpawnAkEventSFX`
  (params (AkEvent :type "AkAudioEvent Object Reference") (SpawnLocation :type "Vector Structure") (FoliageIndex :type Integer)))

(fn `SpawnCascadeVFX`
  (params (CascadeFar :type "ParticleSystem Object Reference") (CascadeClose :type "ParticleSystem Object Reference") (SpawnLocation :type "Vector Structure") (FoliageIndex :type Integer)))

(fn `SpawnEffectsOnFoliageNewLocation`
  (params (Foliage :type "InstancedStaticMeshComponent Object Reference") (InstanceId :type Integer) (FoliageOriginalLocation :type "Vector Structure"))
  (returns (FoliageTransformedLocation :type "Vector Structure"))
  (return (0.0 0.0 0.0)))

(fn `SpawnNiagaraVFX`
  (params (NiagaraFar :type "NiagaraSystem Object Reference") (NiagaraClose :type "NiagaraSystem Object Reference") (SpawnLocation :type "Vector Structure") (ShouldUseFlipBookIndex :type Boolean) (FoliageIndex :type Integer) (FlipBookIndex :type Integer)))

(fn `StartAmbienceTimer`)

(fn `StartDynamicSFXAmbienceTimer`)

(fn `StartWeatherTimer`)

(fn `UpdateQualitySettings`
  (params (Property :type String)))

(fn `UserConstructionScript`)

(fn `WorldAndForwardVector_Func`
  (returns (FoliageRemovalSystem :type "FGFoliageRemovalSubsystem Object Reference") (SpawnLocation_Near :type "Vector Structure") (SpawnLocation_Far :type "Vector Structure"))
  (return null (0.0 0.0 0.0) (0.0 0.0 0.0)))