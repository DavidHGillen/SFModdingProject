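; Player controller Blueprint for FactoryGame, a skeleton exposing hooks for respawn, input gating, photo mode, ragdoll, minimap and dismantling of portable miners and golf carts.
; It holds no logic of its own: several overrides, such as respawn start, photo capture and movement wind setup, only forward to the parent.
; The remaining events and functions are empty stubs, and BeginPlay and Tick are disabled placeholder nodes.
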(event `self.OnStartRespawn`
  (params (isJoining :type Boolean))
  (`parent.OnStartRespawn` isJoining))

(event `CheckAndUpdateGamepad`)

(event `Server_ForceRagdoll`)

(event `self.OnDisabledInputGateChanged`
  (`parent.OnDisabledInputGateChanged`))

(event `self.CreateSequenceList`
  (`parent.CreateSequenceList`))

(event `self.TogglePhotoModeInstructionsWidget`
  (`parent.TogglePhotoModeInstructionsWidget`))

(event `PlayPhotoSound`)

(event `self.TakePhoto`
  (`parent.TakePhoto`))

(event `DoPause`)

(event `self.OnDismantlePortableMiner`
  (params (PortableMiner :type "FGPortableMiner Object Reference"))
  (`parent.OnDismantlePortableMiner` PortableMiner))

(event `self.OnDismantleGolfCart`
  (params (inGolfCart :type "FGWheeledVehicle Object Reference"))
  (`parent.OnDismantleGolfCart` inGolfCart))

(event `OnRespawnFinished`)

(fn `DismantleGolfCart`
  (params (GolfCart :type "FGWheeledVehicle Object Reference")))

(fn `DismantlePortableMiner`
  (params (PortableMiner :type "FGPortableMiner Object Reference")))

(fn `GetPhotoModeWidget`
  (returns (ReturnValue :type "FGPhotoModeWidget Object Reference"))
  (bind _returnvalue (`parent.GetPhotoModeWidget`))
  (return _returnvalue))

(fn `OnDisabledInputChanged`)

(fn `OnSetupMovementWind`
  (returns (ReturnValue :type "AkComponent Object Reference"))
  (bind _returnvalue (`parent.OnSetupMovementWind`))
  (return _returnvalue))

(fn `ToggleMiniMap`)

(fn `UserConstructionScript`)