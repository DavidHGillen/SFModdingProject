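; BP_OnlineHelpers is a shared set of online helper functions covering sessions, friends, presence, invites, host checks and NAT compatibility.
; Every function is a stub: checks return false, the NAT issue text is empty, and visibility parsing returns Private.
; Join and invite checks return a fixed first enum entry, presence getters return no set value, and InsertionAddButton does nothing.
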(fn `CanJoinInviteToSession`
  (params (WorldContext :type "Object Object Reference") (friend :type "FGOnlineFriend Structure") (session :type "BlueprintSessionResult Structure") (invite :type "PendingInvite Structure") (IsFriendOnline :type Boolean))
  (returns (Result :type "/Game/FactoryGame/Interface/UI/Menu/ECanJoinInviteResult Enum"))
  (return "NewEnumerator0"))

(fn `CanSendInvite`
  (params (LocalPlayer :type "LocalPlayer Object Reference") (friend :type "FGOnlineFriend Structure"))
  (returns (canSend :type "/Game/FactoryGame/Interface/UI/Menu/ECantInviteResult Enum"))
  (return "NewEnumerator0"))

(fn `GetCompactPresence`
  (params (presence :type "OnlinePresence Structure"))
  (returns (compactPresence :type "/Game/FactoryGame/-Shared/Blueprint/FCompactPresence Structure"))
  (return))

(fn `GetConnectingNatIssue`
  (params (hostNat :type "ECachedNATType Enum" :default "CNT_Open") (clientNat :type "ECachedNATType Enum" :default "CNT_Open"))
  (returns (ToolTip :type Text))
  (return ""))

(fn `GetFriendPresence`
  (params (onlineFriend :type "FGOnlineFriend Structure (by ref)") (WorldContext :type "Object Object Reference"))
  (returns (ReturnValue :type "OnlinePresence Structure"))
  (return))

(fn `GetInvitePresence`
  (params (WorldContext :type "Object Object Reference") (invite :type "PendingInvite Structure"))
  (returns (presence :type "OnlinePresence Structure"))
  (return))

(fn `InsertionAddButton`
  (params (NewParam :type "PanelWidget Object Reference")))

(fn `IsFriendInPublicSession`
  (params (friend :type "FGOnlineFriend Structure") (WorldContext :type "Object Object Reference"))
  (returns (Result :type Boolean))
  (return false))

(fn `IsFriendInSession`
  (params (friend :type "FGOnlineFriend Structure") (WorldContext :type "Object Object Reference"))
  (returns (Result :type Boolean))
  (return false))

(fn `IsHost`
  (params (PlayerState :type "PlayerState Object Reference") (OwningPlayer :type "PlayerController Object Reference"))
  (returns (isOurself :type Boolean))
  (return false))

(fn `IsInSession`
  (params (presence :type "OnlinePresence Structure"))
  (returns (Result :type Boolean))
  (return false))

(fn `IsInThisGame`
  (params (onlineFriend :type "FGOnlineFriend Structure (by ref)") (LocalPlayer :type "LocalPlayer Object Reference"))
  (returns (inThisGame :type Boolean))
  (return false))

(fn `IsNATIssue`
  (params (hostNat :type "ECachedNATType Enum" :default "CNT_Open") (clientNat :type "ECachedNATType Enum" :default "CNT_Open"))
  (returns (isIssue :type Boolean))
  (return false))

(fn `IsPresenceInPublicSession`
  (params (presence :type "OnlinePresence Structure"))
  (returns (Result :type Boolean))
  (return false))

(fn `SessionVisibilityStringToEnum`
  (params (String :type String))
  (returns (Enum :type "ESessionVisibility Enum"))
  (return "SV_Private"))