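; BP_SchematicHelper is a Blueprint helper with query functions about schematics: their unlocks, recipes and lock states.
; Unlock queries cover inventory slots, hand and arm equipment slots, recipes and unlock data.
; Lock checks cover tutorial, dependency and phase locking, plus a combined check.
; Every function is a stub that returns false, zero or nothing, with no logic or calls between them.
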(fn `DoSchematicHasUnlocks`
  (params (schematic :type "FGSchematic Class Reference"))
  (returns (HasUnlocks :type Boolean))
  (return false))

(fn `GetNumArmEquipmentSlotsUnlocked`
  (params (schematic :type "FGSchematic Class Reference"))
  (returns (numSlots :type Integer))
  (return 0))

(fn `GetNumInventorySlotsUnlocked`
  (params (schematic :type "FGSchematic Class Reference"))
  (returns (numSlots :type Integer))
  (return 0))

(fn `GetRecipesFromSchematic`
  (params (schematic :type "FGSchematic Class Reference"))
  (returns (recipes :type "Array of FGRecipe Class Reference"))
  (return))

(fn `GetUnlockDataStructFromSchematic`
  (params (schematic :type "FGSchematic Class Reference"))
  (returns (UnlockDataStruct :type "Array of /Game/FactoryGame/Unlocks/FUnlockDataStruct Structure"))
  (return))

(fn `GetUnlocksHandSlots`
  (params (schematic :type "FGSchematic Class Reference"))
  (returns (Result :type Boolean))
  (return false))

(fn `GetUnlocksInventorySlot`
  (params (schematic :type "FGSchematic Class Reference"))
  (returns (Result :type Boolean))
  (return false))

(fn `IsSchematicDependentLocked`
  (params (WorldContext :type "Object Object Reference") (SchematicClass :type "FGSchematic Class Reference"))
  (returns (IsSchematicDependentLocked :type Boolean))
  (return false))

(fn `IsSchematicLockedByTutorial`
  (params (WorldContext :type "Object Object Reference") (SchematicClass :type "FGSchematic Class Reference"))
  (returns (IsSchematicLockedByTutorial :type Boolean))
  (return false))

(fn `IsSchematicLockedInAnyWay`
  (params (WolrdContext :type "Object Object Reference") (schematic :type "FGSchematic Class Reference"))
  (returns (IsLocked :type Boolean))
  (return false))

(fn `IsSchematicPartOfTutorial`
  (params (SchematicClass :type "FGSchematic Class Reference"))
  (returns (IsSchematicPartOfTutortial :type Boolean))
  (return false))

(fn `IsSchematicPhaseLocked`
  (params (WorldContext :type "Object Object Reference") (SchematicClass :type "FGSchematic Class Reference"))
  (returns (IsSchematicPhaseLocked :type Boolean))
  (return false))