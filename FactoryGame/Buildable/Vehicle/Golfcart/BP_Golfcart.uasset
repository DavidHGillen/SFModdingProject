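; BP_Golfcart is the Blueprint for the golf cart, a vehicle buildable whose behavior comes almost entirely from its parent class.
; Overrides for possession, honking, free camera, significance, look-at description and dismantle refund only forward to the parent.
; Fold animation, load callback, siren SFX and significance class-check graphs are empty stubs, and BeginPlay, overlap and Tick are disabled placeholders.
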(event `OnLoaded_4386A19442BF0DAA3FC3DEA79644219C`
  (params (Loaded :type "Object Object Reference")))

(event `/Game/FactoryGame/Buildable/Vehicle/BP_WheeledVehicle.ToggleFreeCamera`
  (`parent.ToggleFreeCamera`))

(event `/Game/FactoryGame/Buildable/Vehicle/BP_WheeledVehicle.Multicast_Honk`
  (`parent.Multicast_Honk`))

(event `FoldAnimationDone`)

(event `DoFoldAnimation`)

(event `self.ReceivePossessed`
  (params (NewController :type "Controller Object Reference"))
  (`parent.ReceivePossessed` NewController))

(event `self.ReceiveUnpossessed`
  (params (OldController :type "Controller Object Reference"))
  (`parent.ReceiveUnpossessed` OldController))

(event `FGSignificanceInterface.GainedSignificance`
  (`parent.GainedSignificance`))

(event `FGSignificanceInterface.LostSignificance`
  (`parent.LostSignificance`))

(fn `CheckActorClassOnSignificance`)

(fn `GetDismantleRefund`
  (params (out_refund :type "Array of InventoryStack Structure (by ref)"))
  (`parent.GetDismantleRefund` out_refund)
  (return))

(fn `GetLookAtDecription`
  (params (byCharacter :type "FGCharacterPlayer Object Reference") (state :type "UseState Structure (by ref)"))
  (returns (ReturnValue :type Text))
  (return (`parent.GetLookAtDecription` byCharacter state)))

(fn `PlaySirenSFX`)

(fn `StopSirenSFX`)

(fn `UserConstructionScript`
  (`parent.UserConstructionScript`))