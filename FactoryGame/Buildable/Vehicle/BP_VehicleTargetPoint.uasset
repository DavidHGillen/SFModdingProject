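; Vehicle target point Blueprint, a node with loop target, speed, docking, station, temporary and claimed state, inherited from its parent class.
; Use, look-at, state-change and save overrides only forward to the parent implementation.
; Visual update events, the construction script and Update Visuals are empty, debug mode always returns false, and SelectMode returns a fixed value, leaving the Blueprint without behavior of its own beyond these stubs.
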(event `FGUseableInterface.OnUse`
  (params (byCharacter :type "FGCharacterPlayer Object Reference") (state :type "UseState Structure (by ref)"))
  (`parent.OnUse` byCharacter state))

(event `FGUseableInterface.StartIsLookedAt`
  (params (byCharacter :type "FGCharacterPlayer Object Reference") (state :type "UseState Structure (by ref)"))
  (`parent.StartIsLookedAt` byCharacter state))

(event `FGUseableInterface.StopIsLookedAt`
  (params (byCharacter :type "FGCharacterPlayer Object Reference") (state :type "UseState Structure (by ref)"))
  (`parent.StopIsLookedAt` byCharacter state))

(event `self.IsLoopTargetChanged`
  (`parent.IsLoopTargetChanged`))

(event `self.TargetSpeedChanged`
  (`parent.TargetSpeedChanged`))

(event `self.HostStationChanged`
  (`parent.HostStationChanged`))

(event `self.IsDockingTargetChanged`
  (`parent.IsDockingTargetChanged`))

(event `self.IsTemporaryChanged`
  (`parent.IsTemporaryChanged`))

(event `self.IsClaimedChanged`
  (`parent.IsClaimedChanged`))

(event `UpdateVisualNextFrame`
  (params (NewMesh :type "StaticMesh Object Reference") (Material :type "MaterialInstance Object Reference")))

(event `Update`)

(fn `GatherDependencies`
  (returns (out_dependentObjects :type "Array of Object Object Reference"))
  (bind _out_dependentobjects (`parent.GatherDependencies`))
  (return _out_dependentobjects))

(fn `GetLookAtDecription`
  (params (byCharacter :type "FGCharacterPlayer Object Reference") (state :type "UseState Structure (by ref)"))
  (returns (ReturnValue :type Text))
  (return (`parent.GetLookAtDecription` byCharacter state)))

(fn `IsInDebugMode`
  (returns (ReturnValue :type Boolean))
  (return false))

(fn `IsUseable`
  (returns (ReturnValue :type Boolean))
  (bind _returnvalue (`parent.IsUseable`))
  (return _returnvalue))

(fn `NeedTransform`
  (returns (ReturnValue :type Boolean))
  (bind _returnvalue (`parent.NeedTransform`))
  (return _returnvalue))

(fn `SelectMode`
  (returns (Result :type "/Game/FactoryGame/Buildable/Vehicle/-Shared/EMeshWaypointSelection Enum"))
  (return "NewEnumerator0"))

(fn `ShouldSave`
  (returns (ReturnValue :type Boolean))
  (bind _returnvalue (`parent.ShouldSave`))
  (return _returnvalue))

(fn `Update Visuals`)

(fn `UpdateUseState`
  (params (byCharacter :type "FGCharacterPlayer Object Reference") (atLocation :type "Vector Structure (by ref)") (componentHit :type "PrimitiveComponent Object Reference") (out_useState :type "UseState Structure (by ref)"))
  (`parent.UpdateUseState` byCharacter atLocation componentHit out_useState)
  (return))

(fn `UserConstructionScript`)