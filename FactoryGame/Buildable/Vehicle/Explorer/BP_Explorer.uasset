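; BP_Explorer is the Blueprint for the Explorer vehicle, containing almost no logic of its own.
; Significance, trunk multicast, outline and enemy-targeting overrides simply forward to the parent class, which supplies the actual behavior.
; Flashlight replication and server RPC, suspension check and forward-axis input are empty stubs, while BeginPlay, Tick and overlap events are disabled.
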(event `FGSignificanceInterface.GainedSignificance`
  (`parent.GainedSignificance`))

(event `FGSignificanceInterface.LostSignificance`
  (`parent.LostSignificance`))

(event `/Game/FactoryGame/Buildable/Vehicle/BP_WheeledVehicle.Multicast_OpenTrunk`
  (`parent.Multicast_OpenTrunk`))

(event `/Game/FactoryGame/Buildable/Vehicle/BP_WheeledVehicle.Multicast_CloseTrunk`
  (`parent.Multicast_CloseTrunk`))

(event `Server_SetFlashlightOn`
  (params (FlashlightOn :type Boolean)))

(event `InpAxisEvt_MoveForward_K2Node_InputAxisEvent_0`
  (params (AxisValue :type "Float (double-precision)")))

(fn `CheckSuspension`
  (params (InDeltaTime :type "Float (double-precision)")))

(fn `GetAttackLocation`
  (returns (ReturnValue :type "Vector Structure"))
  (return (`parent.GetAttackLocation`)))

(fn `GetEnemyTargetDesirability`
  (params (forController :type "FGEnemyController Object Reference"))
  (returns (ReturnValue :type "Float (double-precision)"))
  (bind _returnvalue (`parent.GetEnemyTargetDesirability` forController))
  (return _returnvalue))

(fn `OnRep_mFlashlightOn`)

(fn `ShouldAutoregisterAsTargetable`
  (returns (ReturnValue :type Boolean))
  (bind _returnvalue (`parent.ShouldAutoregisterAsTargetable`))
  (return _returnvalue))

(fn `UpdateOutline`
  (params (aimingAtWorkbench :type Boolean))
  (`parent.UpdateOutline` aimingAtWorkbench))

(fn `UserConstructionScript`
  (`parent.UserConstructionScript`))