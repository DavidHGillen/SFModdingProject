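; Tractor vehicle Blueprint whose graphs add almost no logic of their own.
; Startup, shutdown, free camera, trunk, significance, outline and enemy-targeting overrides simply forward to the parent class.
; Flashlight and driving-effect overrides are empty and make no parent call, and the Tick and overlap events are disabled.
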(event `self.ReceiveBeginPlay`
  (`parent.ReceiveBeginPlay`))

(event `/Game/FactoryGame/Buildable/Vehicle/BP_WheeledVehicle.ToggleFreeCamera`
  (`parent.ToggleFreeCamera`))

(event `self.ReceiveOnVehicleStartup`
  (`parent.ReceiveOnVehicleStartup`))

(event `self.ReceiveOnVehicleShutDown`
  (`parent.ReceiveOnVehicleShutDown`))

(event `Server_SetFlashlightOn`
  (params (FlashlightOn :type Boolean)))

(event `FGSignificanceInterface.GainedSignificance`
  (`parent.GainedSignificance`))

(event `FGSignificanceInterface.LostSignificance`
  (`parent.LostSignificance`))

(event `/Game/FactoryGame/Buildable/Vehicle/BP_WheeledVehicle.Multicast_CloseTrunk`
  (`parent.Multicast_CloseTrunk`))

(event `/Game/FactoryGame/Buildable/Vehicle/BP_WheeledVehicle.Multicast_OpenTrunk`
  (`parent.Multicast_OpenTrunk`))

(fn `GetAttackLocation`
  (returns (ReturnValue :type "Vector Structure"))
  (return (`parent.GetAttackLocation`)))

(fn `GetEnemyTargetDesirability`
  (params (forController :type "FGEnemyController Object Reference"))
  (returns (ReturnValue :type "Float (double-precision)"))
  (bind _returnvalue (`parent.GetEnemyTargetDesirability` forController))
  (return _returnvalue))

(fn `OnRep_mFlashlightOn`)

(fn `ShouldAutoregisterAsTargetable`
  (returns (ReturnValue :type Boolean))
  (bind _returnvalue (`parent.ShouldAutoregisterAsTargetable`))
  (return _returnvalue))

(fn `StartDrivingEffects`)

(fn `StopDrivingEffects`)

(fn `ToggleFlashlight`)

(fn `UpdateOutline`
  (params (aimingAtWorkbench :type Boolean))
  (`parent.UpdateOutline` aimingAtWorkbench))

(fn `UserConstructionScript`
  (`parent.UserConstructionScript`))