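; BP_Truck is the truck vehicle Blueprint, a child class that leaves almost all behavior to its parent.
; Significance, trunk, load/unload, outline and enemy-targeting overrides only forward to the parent implementation.
; Storage sound, montage, state-seek and flashlight functions are empty stubs, as are the leftover montage notify callbacks.
; BeginPlay, overlap and Tick nodes are disabled, so the graphs add no logic of their own.
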(event `OnNotifyEnd_0C5D05504ED095AA6118B99B99D9EDC2`
  (params (NotifyName :type Name)))

(event `OnNotifyBegin_0C5D05504ED095AA6118B99B99D9EDC2`
  (params (NotifyName :type Name)))

(event `OnInterrupted_0C5D05504ED095AA6118B99B99D9EDC2`
  (params (NotifyName :type Name)))

(event `OnBlendOut_0C5D05504ED095AA6118B99B99D9EDC2`
  (params (NotifyName :type Name)))

(event `OnCompleted_0C5D05504ED095AA6118B99B99D9EDC2`
  (params (NotifyName :type Name)))

(event `OnNotifyEnd_55FDF12A4940D1ECC665FC8A0684A3E4`
  (params (NotifyName :type Name)))

(event `OnNotifyBegin_55FDF12A4940D1ECC665FC8A0684A3E4`
  (params (NotifyName :type Name)))

(event `OnInterrupted_55FDF12A4940D1ECC665FC8A0684A3E4`
  (params (NotifyName :type Name)))

(event `OnBlendOut_55FDF12A4940D1ECC665FC8A0684A3E4`
  (params (NotifyName :type Name)))

(event `OnCompleted_55FDF12A4940D1ECC665FC8A0684A3E4`
  (params (NotifyName :type Name)))

(event `FGSignificanceInterface.GainedSignificance`
  (`parent.GainedSignificance`))

(event `FGSignificanceInterface.LostSignificance`
  (`parent.LostSignificance`))

(event `/Game/FactoryGame/Buildable/Vehicle/BP_WheeledVehicle.Multicast_OpenTrunk`
  (`parent.Multicast_OpenTrunk`))

(event `/Game/FactoryGame/Buildable/Vehicle/BP_WheeledVehicle.Multicast_CloseTrunk`
  (`parent.Multicast_CloseTrunk`))

(event `FGDockableInterface.OnBeginLoadVehicle`
  (`parent.OnBeginLoadVehicle`))

(event `FGDockableInterface.OnBeginUnloadVehicle`
  (`parent.OnBeginUnloadVehicle`))

(event `Server_SetFlashlightOn`
  (params (FlashlightOn :type Boolean)))

(fn `CheckCurrentActiveMontage`)

(fn `FindAttachedStaticMesh`
  (returns (ReturnValue :type "StaticMesh Object Reference"))
  (bind _returnvalue (`parent.FindAttachedStaticMesh`))
  (return _returnvalue))

(fn `GetAttackLocation`
  (returns (ReturnValue :type "Vector Structure"))
  (return (`parent.GetAttackLocation`)))

(fn `GetEnemyTargetDesirability`
  (params (forController :type "FGEnemyController Object Reference"))
  (returns (ReturnValue :type "Float (double-precision)"))
  (bind _returnvalue (`parent.GetEnemyTargetDesirability` forController))
  (return _returnvalue))

(fn `OnRep_mFlashlightOn`)

(fn `PlayCloseStorageSFX`)

(fn `PlayOpenStorageSFX`)

(fn `SeekIntoCurrentState`)

(fn `ShouldAutoregisterAsTargetable`
  (returns (ReturnValue :type Boolean))
  (bind _returnvalue (`parent.ShouldAutoregisterAsTargetable`))
  (return _returnvalue))

(fn `UpdateOutline`
  (params (aimingAtWorkbench :type Boolean))
  (`parent.UpdateOutline` aimingAtWorkbench))

(fn `UserConstructionScript`
  (`parent.UserConstructionScript`))