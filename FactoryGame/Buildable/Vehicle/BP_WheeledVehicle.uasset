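; Blueprint base for wheeled vehicles in FactoryGame, consisting almost entirely of stubs and pass-throughs to its parent class.
; Lifecycle, possession, use, hit, trunk open/close, camera and path-following events only forward to the parent implementation.
; Input axes, honk and trunk multicasts, gear checks, engine and tire sound functions, outline and UI hooks are empty, so the graphs add no logic of their own.
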(event `self.ReceiveBeginPlay`
  (`parent.ReceiveBeginPlay`))

(event `self.ReceiveTick`
  (params (DeltaSeconds :type "Float (single-precision)"))
  (`parent.ReceiveTick` DeltaSeconds))

(event `TickVehicleSound`
  (params (dt :type "Float (double-precision)")))

(event `self.ReceiveUnpossessed`
  (params (OldController :type "Controller Object Reference"))
  (`parent.ReceiveUnpossessed` OldController))

(event `self.ReceiveHit`
  (params (MyComp :type "PrimitiveComponent Object Reference") (Other :type "Actor Object Reference") (OtherComp :type "PrimitiveComponent Object Reference") (bSelfMoved :type Boolean) (HitLocation :type "Vector Structure") (HitNormal :type "Vector Structure") (NormalImpulse :type "Vector Structure") (Hit :type "HitResult Structure (by ref)"))
  (`parent.ReceiveHit` MyComp Other OtherComp bSelfMoved HitLocation HitNormal NormalImpulse Hit))

(event `self.ReceiveDestroyed`
  (`parent.ReceiveDestroyed`))

(event `ResetImpactSound`)

(event `FGUseableInterface.OnUse`
  (params (byCharacter :type "FGCharacterPlayer Object Reference") (state :type "UseState Structure (by ref)"))
  (`parent.OnUse` byCharacter state))

(event `Multicast_OpenTrunk`)

(event `Multicast_CloseTrunk`)

(event `self.ReceivePossessed`
  (params (NewController :type "Controller Object Reference"))
  (`parent.ReceivePossessed` NewController))

(event `StartAccelerating`)

(event `StopAccelerating`)

(event `self.ReceiveOnVehicleStartup`
  (`parent.ReceiveOnVehicleStartup`))

(event `self.ReceiveOnVehicleShutDown`
  (`parent.ReceiveOnVehicleShutDown`))

(event `InpAxisEvt_MoveForward_K2Node_InputAxisEvent_1`
  (params (AxisValue :type "Float (double-precision)")))

(event `InpAxisEvt_MoveRight_K2Node_InputAxisEvent_2`
  (params (AxisValue :type "Float (double-precision)")))

(event `Server_Honk`)

(event `Multicast_Honk`)

(event `self.Client_PlayFoliageDestroyedEffect`
  (params (destroyEffect :type "ParticleSystem Object Reference") (destroyAudioEvent :type "AkAudioEvent Object Reference") (location :type "Vector Structure"))
  (`parent.Client_PlayFoliageDestroyedEffect` destroyEffect destroyAudioEvent location))

(event `self.OpenVehicleTrunk`
  (params (player :type "FGCharacterPlayer Object Reference"))
  (`parent.OpenVehicleTrunk` player))

(event `self.CloseVehicleTrunk`
  (params (player :type "FGCharacterPlayer Object Reference"))
  (`parent.CloseVehicleTrunk` player))

(event `self.UpdateCamera`
  (params (DeltaTime :type "Float (single-precision)"))
  (`parent.UpdateCamera` DeltaTime))

(event `self.IsFollowingPathChanged`
  (params (isFollowingPath :type Boolean))
  (`parent.IsFollowingPathChanged` isFollowingPath))

(event `InpAxisEvt_Turn_K2Node_InputAxisEvent_0`
  (params (AxisValue :type "Float (double-precision)")))

(fn `BurnOutSound`
  (params (ForwardInputInput :type "Float (double-precision)")))

(fn `CheckCurrentGear`)

(fn `DidGearDown`)

(fn `DidGearUp`)

(fn `GetDefaultRepresentationColor`
  (returns (ReturnValue :type "LinearColor Structure"))
  (bind _returnvalue (`parent.GetDefaultRepresentationColor`))
  (return _returnvalue))

(fn `GetDriftForceOffset`
  (returns (ReturnValue :type "Vector Structure"))
  (bind _returnvalue (`parent.GetDriftForceOffset`))
  (return _returnvalue))

(fn `GetLookAtDecription`
  (params (byCharacter :type "FGCharacterPlayer Object Reference") (state :type "UseState Structure (by ref)"))
  (returns (ReturnValue :type Text))
  (return (`parent.GetLookAtDecription` byCharacter state)))

(fn `OpenVehicleUI`
  (params (inCharacter :type "FGCharacterPlayer Object Reference")))

(fn `PonderOpeningTrunk`
  (params (inCharacter :type "FGCharacterPlayer Object Reference")))

(fn `StartSoundLoops`)

(fn `StopSoundLoops`)

(fn `ToggleFreeCamera`)

(fn `UpdateAccelerationSound`)

(fn `UpdateAudioGear`)

(fn `UpdateEngineLoadSound`
  (params (dt :type "Float (double-precision)")))

(fn `UpdateOutline`
  (params (aimingAtWorkbench :type Boolean)))

(fn `UpdateThrottleState`)

(fn `UpdateTireSound`)

(fn `UpdateUseState`
  (params (byCharacter :type "FGCharacterPlayer Object Reference") (atLocation :type "Vector Structure (by ref)") (componentHit :type "PrimitiveComponent Object Reference") (out_useState :type "UseState Structure (by ref)"))
  (`parent.UpdateUseState` byCharacter atLocation componentHit out_useState)
  (return))

(fn `UserConstructionScript`)