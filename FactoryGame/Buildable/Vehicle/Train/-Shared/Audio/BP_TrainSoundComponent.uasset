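; Base train sound component Blueprint exposing hooks for movement, throttle, air and dynamic brakes, and idle or stop-all sound control.
; Almost every event simply forwards to its parent implementation, so the graph adds no audio logic of its own.
; OnStoppedMovingRelay is empty, BeginPlay and Tick are disabled, and SpeedKmH is a stub that returns zero.
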(event `self.OnThrottleReleased`
  (`parent.OnThrottleReleased`))

(event `self.OnThrottleApplied`
  (`parent.OnThrottleApplied`))

(event `self.OnDynamicBrakesReleased`
  (`parent.OnDynamicBrakesReleased`))

(event `self.OnAirBrakesReleased`
  (`parent.OnAirBrakesReleased`))

(event `OnStoppedMovingRelay`)

(event `self.OnAirBrakesApplied`
  (`parent.OnAirBrakesApplied`))

(event `self.StartIdleSounds`
  (`parent.StartIdleSounds`))

(event `self.StopAllSounds`
  (`parent.StopAllSounds`))

(event `self.OnDynamicBrakesApplied`
  (`parent.OnDynamicBrakesApplied`))

(event `self.OnStartedMoving`
  (`parent.OnStartedMoving`))

(event `self.OnStoppedMoving`
  (`parent.OnStoppedMoving`))

(fn `SpeedKmH`
  (returns (Speed :type "Float (double-precision)"))
  (return 0.0))