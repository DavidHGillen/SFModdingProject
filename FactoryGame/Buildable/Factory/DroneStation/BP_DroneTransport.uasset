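; Blueprint for the transport drone that docks at and takes off from drone stations.
; Flight, braking, docking, significance and VFX tick events only forward to the parent class, which supplies the behavior.
; The many functions and events for thruster and fan VFX, sounds, and docking animations are empty stubs, leaving this Blueprint with no logic of its own.
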(event `self.ReceiveBeginPlay`
  (`parent.ReceiveBeginPlay`))

(event `self.ReceiveTick`
  (params (DeltaSeconds :type "Float (single-precision)"))
  (`parent.ReceiveTick` DeltaSeconds))

(event `self.OnFlyingModeChanged`
  (params (NewMode :type "EDroneFlyingMode Enum" :default "DFM_None"))
  (`parent.OnFlyingModeChanged` NewMode))

(event `self.StartDockingSequence`
  (params (Station :type "FGBuildableDroneStation Object Reference"))
  (`parent.StartDockingSequence` Station))

(event `self.StartTakeoffSequence`
  (params (Station :type "FGBuildableDroneStation Object Reference"))
  (`parent.StartTakeoffSequence` Station))

(event `DockingTimerEvent`)

(event `TakeOffTimerEvent`)

(event `self.OnBrakingStateChanged`
  (params (IsBraking :type Boolean))
  (`parent.OnBrakingStateChanged` IsBraking))

(event `FGSignificanceInterface.GainedSignificance`
  (`parent.GainedSignificance`))

(event `FGSignificanceInterface.LostSignificance`
  (`parent.LostSignificance`))

(event `TickForDrone`)

(event `/Game/FactoryGame/Buildable/Factory/DroneStation/BPI_Drone.Start_FX`)

(event `/Game/FactoryGame/Buildable/Factory/DroneStation/BPI_Drone.Deactivate_FX`)

(event `TickForDeactivateDrone`)

(event `self.OnDockingStateChanged`
  (params (NewState :type "EDroneDockingState Enum" :default "DS_UNDOCKED") (TimeSinceChanged :type "Float (single-precision)"))
  (`parent.OnDockingStateChanged` NewState TimeSinceChanged))

(event `TickForThrusters`)

(event `StartThrusters`)

(event `self.TickVFX`
  (`parent.TickVFX`))

(event `self.ReceiveDestroyed`
  (`parent.ReceiveDestroyed`))

(event `UpdateThrusterRate`)

(event `TurnOffThrusters`)

(event `TickForTurnOffThrusters`)

(fn `CheckDecendingStatusSound`)

(fn `CheckTakeOffStatusSound`)

(fn `DecendingBrakeSound`)

(fn `GainSignificanceSound`)

(fn `GetDefaultRepresentationColor`
  (returns (ReturnValue :type "LinearColor Structure"))
  (bind _returnvalue (`parent.GetDefaultRepresentationColor`))
  (return _returnvalue))

(fn `KillCurrentMontage`)

(fn `KillFan_VFX`)

(fn `KillThruster_VFX`)

(fn `LostSignificanceSound`)

(fn `OnFlyingModeChange`
  (params (NewFlyingMode :type "EDroneFlyingMode Enum" :default "DFM_None") (NewParam1 :type Byte))
  (returns (NewParam :type Byte))
  (return 0))

(fn `PlayBlastOffSound`)

(fn `PlayDockingAnimationAndTime`
  (params (mTime :type "Float (double-precision)")))

(fn `PlayDockingPlatformSound`
  (params (Time :type "Float (double-precision)")))

(fn `PlayDockingSoundSequence`
  (params (Time :type "Float (double-precision)")))

(fn `PlayTakeOffAnimationAndTime`
  (params (mTime :type "Float (double-precision)")))

(fn `PlayTakeOffPlatformSound`
  (params (Time :type "Float (double-precision)")))

(fn `PlayTakeOffSoundSequence`
  (params (Time :type "Float (double-precision)")))

(fn `SetThrusterMesh_Values_VFX`)

(fn `SpawnFan_VFX`)

(fn `SpawnThruster_VFX`)

(fn `StopBlastOffSound`)

(fn `TriggerAnimationDockingBool`)

(fn `TriggerAnimationTakeOffBool`)

(fn `TurnOffAllThrusters`
  (params (Float :type "Float (double-precision)")))

(fn `UpdateFan_VFX`
  (params (Float :type "Float (double-precision)") (bAleadyFlying :type Boolean) (bReveresed :type Boolean)))

(fn `UpdateThruster_VFX`
  (params (Float :type "Float (double-precision)") (bAleadyFlying :type Boolean) (bReveresed :type Boolean)))

(fn `UserConstructionScript`)