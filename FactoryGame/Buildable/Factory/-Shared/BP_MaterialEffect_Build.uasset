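; BP_MaterialEffect_Build is a shared factory buildable Blueprint, named as the material effect for building.
; Its update, start, pre-start and end events only forward to the parent class.
; All other events and functions are empty stubs or return zero, including those named for cost queue, meshes, bounds, displacement, thump sound and foot emitters, so the graphs shown add no behavior of their own.
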(event `self.OnUpdate`
  (params (deltaTime :type "Float (single-precision)"))
  (`parent.OnUpdate` deltaTime))

(event `self.OnEnded`
  (`parent.OnEnded`))

(event `self.PreStarted`
  (`parent.PreStarted`))

(event `self.OnStarted`
  (`parent.OnStarted`))

(event `OnCostActorReachedTarget`)

(event `destroy proxies`)

(fn `CalcCostQueueNewLength`
  (returns (NewLength :type Integer))
  (return 0))

(fn `CalcDisplacementAmount`
  (returns (Amount :type "Float (double-precision)"))
  (return 0.0))

(fn `DebugFillCostQueue`)

(fn `GotoNextStep`)

(fn `InitMaterialParameters`)

(fn `PlayThumpSound`)

(fn `SetupBounds`)

(fn `SetupCostQueue`)

(fn `SetupDuration`)

(fn `SetupMeshes`)

(fn `setupNormal`)

(fn `SpawnFootEmitters`)

(fn `UpdateCostQueue`)