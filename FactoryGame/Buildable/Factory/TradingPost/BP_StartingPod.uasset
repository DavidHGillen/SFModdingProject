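; BP_StartingPod is the starting pod Blueprint, with event hooks for an intro cinematic, owner and observer setup, intro skipping and audio ducking.
; Nearly all of these hooks are empty stubs; lifecycle, dismantle look-at, intro-skip notification and representation color only forward to the parent class.
; Its save interface returns false for both ShouldSave and NeedTransform, so the pod is excluded from save games.
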(event `self.ReceiveBeginPlay`
  (`parent.ReceiveBeginPlay`))

(event `self.ReceiveTick`
  (params (DeltaSeconds :type "Float (single-precision)"))
  (`parent.ReceiveTick` DeltaSeconds))

(event `OnLoaded_8586F6D040F0FFE03962849F398DB59A`
  (params (Loaded :type "Object Object Reference")))

(event `FGSaveInterface.PostLoadGame`
  (params (saveVersion :type Integer) (gameVersion :type Integer)))

(event `FGSaveInterface.PostSaveGame`
  (params (saveVersion :type Integer) (gameVersion :type Integer)))

(event `FGSaveInterface.PreLoadGame`
  (params (saveVersion :type Integer) (gameVersion :type Integer)))

(event `FGSaveInterface.PreSaveGame`
  (params (saveVersion :type Integer) (gameVersion :type Integer)))

(event `FGDismantleInterface.StartIsLookedAtForDismantle`
  (params (byCharacter :type "FGCharacterPlayer Object Reference"))
  (`parent.StartIsLookedAtForDismantle` byCharacter))

(event `FGDismantleInterface.StopIsLookedAtForDismantle`
  (params (byCharacter :type "FGCharacterPlayer Object Reference"))
  (`parent.StopIsLookedAtForDismantle` byCharacter))

(event `SetupPodForOwner`)

(event `SetupPodForObserver`)

(event `EndCinematic`)

(event `StartMovie`)

(event `AK_StopDucking`)

(event `AK_HalveDucking`)

(event `self.ReceiveDestroyed`
  (`parent.ReceiveDestroyed`))

(event `StartCinematic`)

(event `self.OnPlayerSkipIntroSequence`
  (`parent.OnPlayerSkipIntroSequence`))

(event `AllowSkipIntro`)

(event `BlockSkipIntro`)

(fn `GatherDependencies`
  (returns (out_dependentObjects :type "Array of Object Object Reference"))
  (return))

(fn `GetDefaultRepresentationColor`
  (returns (ReturnValue :type "LinearColor Structure"))
  (bind _returnvalue (`parent.GetDefaultRepresentationColor`))
  (return _returnvalue))

(fn `NeedTransform`
  (returns (ReturnValue :type Boolean))
  (return false))

(fn `ShouldSave`
  (returns (ReturnValue :type Boolean))
  (return false))

(fn `UserConstructionScript`)