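; Blueprint build gun state for painting, which applies swatch, pattern and material customizations to buildings.
; Its events cover state begin and end, secondary fire, descriptor changes, hit validity and customization success or failure, and each only calls the parent implementation.
; OpenCustomiserUI is an empty stub, so this graph adds no behavior of its own.
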(event `OpenCustomiserUI`)

(event `self.EndState`
  (`parent.EndState`))

(event `self.OnMaterialDescriptorChanged`
  (params (newMaterialDesc :type "FGFactoryCustomizationDescriptor_Material Class Reference"))
  (`parent.OnMaterialDescriptorChanged` newMaterialDesc))

(event `self.OnPatternDescriptorChanged`
  (params (newPatternDesc :type "FGFactoryCustomizationDescriptor_Pattern Class Reference"))
  (`parent.OnPatternDescriptorChanged` newPatternDesc))

(event `self.OnSwatchDescriptorChanged`
  (params (newColorDesc :type "FGFactoryCustomizationDescriptor_Swatch Class Reference"))
  (`parent.OnSwatchDescriptorChanged` newColorDesc))

(event `self.OnHitStatusChanged`
  (params (hitBuildingDesc :type "FGBuildingDescriptor Class Reference") (validSwatch :type Boolean) (validPattern :type Boolean) (validMaterial :type Boolean))
  (`parent.OnHitStatusChanged` hitBuildingDesc validSwatch validPattern validMaterial))

(event `self.SecondaryFire`
  (`parent.SecondaryFire`))

(event `self.BeginState`
  (`parent.BeginState`))

(event `self.OnApplyCustomization`
  (params (customizationDesc :type "FGFactoryCustomizationDescriptor Class Reference"))
  (`parent.OnApplyCustomization` customizationDesc))

(event `self.OnApplyCustomizationFailed`
  (`parent.OnApplyCustomizationFailed`))