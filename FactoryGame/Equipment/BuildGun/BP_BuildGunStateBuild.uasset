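; BP_BuildGunStateBuild is the Blueprint for the build gun's build state, covering events for placing buildables through a hologram.
; It adds no logic of its own: the overridden state, fire, scroll, recipe sampling, zoop, hologram reset and multi-step placement events only forward to the parent.
; The build mode select UI events also pass through to the parent, while OpenBuildModeUI is an empty stub.
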(event `self.SecondaryFire`
  (`parent.SecondaryFire`))

(event `self.PrimaryFire`
  (`parent.PrimaryFire`))

(event `self.EndState`
  (`parent.EndState`))

(event `self.BeginState`
  (`parent.BeginState`))

(event `OpenBuildModeUI`)

(event `self.OnRecipeSampled`
  (params (recipe :type "FGRecipe Class Reference"))
  (`parent.OnRecipeSampled` recipe))

(event `self.ShowBuildModeSelectUI`
  (`parent.ShowBuildModeSelectUI`))

(event `self.CloseBuildModeSelectUI`
  (`parent.CloseBuildModeSelectUI`))

(event `self.OnZoopUpdated`
  (params (currentZoop :type "Float (single-precision)") (maxZoop :type "Float (single-precision)") (zoopLocation :type "Vector Structure (by ref)"))
  (`parent.OnZoopUpdated` currentZoop maxZoop zoopLocation))

(event `self.ScrollDown`
  (`parent.ScrollDown`))

(event `self.ScrollUp`
  (`parent.ScrollUp`))

(event `self.OnResetHologram`
  (`parent.OnResetHologram`))

(event `self.OnMultiStepPlacement`
  (params (isFinalStep :type Boolean))
  (`parent.OnMultiStepPlacement` isFinalStep))