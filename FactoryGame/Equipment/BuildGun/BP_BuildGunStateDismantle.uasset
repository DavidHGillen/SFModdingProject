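; BP_BuildGunStateDismantle is the Blueprint build gun state for dismantling.
; Its event graph overrides state begin, end and tick, secondary fire, dismantle start and stop, and recipe sampling.
; Each override only forwards to its parent implementation, so the graph adds no behavior of its own.
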(event `self.TickState`
  (params (deltaTime :type "Float (single-precision)"))
  (`parent.TickState` deltaTime))

(event `self.SecondaryFire`
  (`parent.SecondaryFire`))

(event `self.BeginState`
  (`parent.BeginState`))

(event `self.EndState`
  (`parent.EndState`))

(event `self.OnStartDismantle`
  (`parent.OnStartDismantle`))

(event `self.OnStopDismantle`
  (`parent.OnStopDismantle`))

(event `self.OnRecipeSampled`
  (params (recipe :type "FGRecipe Class Reference"))
  (`parent.OnRecipeSampled` recipe))