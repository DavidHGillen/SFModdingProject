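; BP_Beacon is a beacon actor that can be picked up and carries a text, color and compass view distance for its representation.
; BeginPlay, pickup and the representation getters and setters only forward to parent implementations.
; Save, interaction, SetColor, widget and planted-sound functions are empty stubs or return defaults, with IsUseable and ShouldSave both false.
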(event `self.ReceiveBeginPlay`
  (`parent.ReceiveBeginPlay`))

(event `FGSaveInterface.PostLoadGame`
  (params (saveVersion :type Integer) (gameVersion :type Integer)))

(event `FGSaveInterface.PostSaveGame`
  (params (saveVersion :type Integer) (gameVersion :type Integer)))

(event `FGSaveInterface.PreLoadGame`
  (params (saveVersion :type Integer) (gameVersion :type Integer)))

(event `FGSaveInterface.PreSaveGame`
  (params (saveVersion :type Integer) (gameVersion :type Integer)))

(event `FGUseableInterface.OnUseStop`
  (params (byCharacter :type "FGCharacterPlayer Object Reference") (state :type "UseState Structure (by ref)")))

(event `FGUseableInterface.RegisterInteractingPlayer`
  (params (player :type "FGCharacterPlayer Object Reference")))

(event `FGUseableInterface.StartIsLookedAt`
  (params (byCharacter :type "FGCharacterPlayer Object Reference") (state :type "UseState Structure (by ref)")))

(event `FGUseableInterface.StopIsLookedAt`
  (params (byCharacter :type "FGCharacterPlayer Object Reference") (state :type "UseState Structure (by ref)")))

(event `FGUseableInterface.UnregisterInteractingPlayer`
  (params (player :type "FGCharacterPlayer Object Reference")))

(event `FGUseableInterface.OnUse`
  (params (byCharacter :type "FGCharacterPlayer Object Reference") (state :type "UseState Structure (by ref)")))

(event `self.PickUpBeacon`
  (params (player :type "FGCharacterPlayer Object Reference"))
  (`parent.PickUpBeacon` player))

(event `self.SetRepresentationText`
  (params (text :type "Text (by ref)"))
  (`parent.SetRepresentationText` text))

(event `self.SetCompassViewDistance`
  (params (compassViewDistance :type "ECompassViewDistance Enum" :default "CVD_Off"))
  (`parent.SetCompassViewDistance` compassViewDistance))

(event `self.SetRepresentationColor`
  (params (color :type "LinearColor Structure (by ref)"))
  (`parent.SetRepresentationColor` color))

(fn `CloseWidget`
  (params (Controller :type "Controller Object Reference")))

(fn `GatherDependencies`
  (returns (out_dependentObjects :type "Array of Object Object Reference"))
  (return))

(fn `GetCompassViewDistance`
  (returns (ReturnValue :type "ECompassViewDistance Enum"))
  (bind _returnvalue (`parent.GetCompassViewDistance`))
  (return _returnvalue))

(fn `GetLookAtDecription`
  (params (byCharacter :type "FGCharacterPlayer Object Reference") (state :type "UseState Structure (by ref)"))
  (returns (ReturnValue :type Text))
  (return ""))

(fn `GetRepresentationColor`
  (returns (ReturnValue :type "LinearColor Structure"))
  (bind _returnvalue (`parent.GetRepresentationColor`))
  (return _returnvalue))

(fn `GetRepresentationText`
  (returns (ReturnValue :type Text))
  (bind _returnvalue (`parent.GetRepresentationText`))
  (return _returnvalue))

(fn `IsUseable`
  (returns (ReturnValue :type Boolean))
  (return false))

(fn `NeedTransform`
  (returns (ReturnValue :type Boolean))
  (return false))

(fn `SetColor`
  (params (NewColor :type "LinearColor Structure")))

(fn `ShouldSave`
  (returns (ReturnValue :type Boolean))
  (return false))

(fn `StopPlantedSFXIfValid`)

(fn `UpdateUseState`
  (params (byCharacter :type "FGCharacterPlayer Object Reference") (atLocation :type "Vector Structure (by ref)") (componentHit :type "PrimitiveComponent Object Reference") (out_useState :type "UseState Structure (by ref)"))
  (return))

(fn `UserConstructionScript`)