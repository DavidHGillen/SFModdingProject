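; Boombox actor Blueprint whose events and overrides cover tape selection, song controls, pickup and player interaction, almost all left empty.
; BeginPlay, EndPlay, OnDistanceChanged and IsPlaying only forward to the parent class.
; The use and look-at overrides are stubbed: IsUseable returns false, the description is blank, and the pickup and data replication handlers do nothing.
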(event `self.ReceiveBeginPlay`
  (`parent.ReceiveBeginPlay`))

(event `/Game/FactoryGame/Equipment/BoomBox/BPI_BoomBox.OnTapeSelected`
  (params (newTape :type "FGTapeDescriptor Class Reference")))

(event `/Game/FactoryGame/Equipment/BoomBox/BPI_BoomBox.NextSongPressed`)

(event `/Game/FactoryGame/Equipment/BoomBox/BPI_BoomBox.PreviousSongPressed`)

(event `/Game/FactoryGame/Equipment/BoomBox/BPI_BoomBox.ToggleBassPressed`)

(event `FGUseableInterface.OnUseStop`
  (params (byCharacter :type "FGCharacterPlayer Object Reference") (state :type "UseState Structure (by ref)")))

(event `FGUseableInterface.RegisterInteractingPlayer`
  (params (player :type "FGCharacterPlayer Object Reference")))

(event `FGUseableInterface.StartIsLookedAt`
  (params (byCharacter :type "FGCharacterPlayer Object Reference") (state :type "UseState Structure (by ref)")))

(event `FGUseableInterface.StopIsLookedAt`
  (params (byCharacter :type "FGCharacterPlayer Object Reference") (state :type "UseState Structure (by ref)")))

(event `FGUseableInterface.UnregisterInteractingPlayer`
  (params (player :type "FGCharacterPlayer Object Reference")))

(event `FGUseableInterface.OnUse`
  (params (byCharacter :type "FGCharacterPlayer Object Reference") (state :type "UseState Structure (by ref)")))

(event `/Game/FactoryGame/Equipment/BoomBox/BPI_BoomBox.SongFinished`
  (params (CallbackType :type "EAkCallbackType Enum" :default "EndOfEvent") (CallbackInfo :type "AkCallbackInfo Object Reference")))

(event `self.ReceiveEndPlay`
  (params (EndPlayReason :type "EEndPlayReason Enum" :default "Destroyed"))
  (`parent.ReceiveEndPlay` EndPlayReason))

(event `FGMusicPlayerInterface.OnDistanceChanged`
  (params (distSquared :type "Float (single-precision)") (isClosest :type Boolean))
  (`parent.OnDistanceChanged` distSquared isClosest))

(fn `GetLookAtDecription`
  (params (byCharacter :type "FGCharacterPlayer Object Reference") (state :type "UseState Structure (by ref)"))
  (returns (ReturnValue :type Text))
  (return ""))

(fn `IsPlaying`
  (returns (ReturnValue :type Boolean))
  (bind _returnvalue (`parent.IsPlaying`))
  (return _returnvalue))

(fn `IsUseable`
  (returns (ReturnValue :type Boolean))
  (return false))

(fn `OnRep_mBoomBoxData`)

(fn `PickUpBoomBox`
  (params (inPlayer :type "FGCharacterPlayer Object Reference")))

(fn `UpdateUseState`
  (params (byCharacter :type "FGCharacterPlayer Object Reference") (atLocation :type "Vector Structure (by ref)") (componentHit :type "PrimitiveComponent Object Reference") (out_useState :type "UseState Structure (by ref)"))
  (return))

(fn `UserConstructionScript`)