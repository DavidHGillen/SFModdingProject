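; Base Blueprint for a decoration actor in the equipment system, with hooks for use, look-at text and saving.
; BeginPlay, OnUse and the save and use-state overrides only forward to the parent class, so behavior comes from the parent.
; SetupActor, PickUp and the construction script are empty, adding no logic of their own.
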(event `self.ReceiveBeginPlay`
  (`parent.ReceiveBeginPlay`))

(event `FGUseableInterface.OnUse`
  (params (byCharacter :type "FGCharacterPlayer Object Reference") (state :type "UseState Structure (by ref)"))
  (`parent.OnUse` byCharacter state))

(event `SetupActor`)

(fn `GatherDependencies`
  (returns (out_dependentObjects :type "Array of Object Object Reference"))
  (bind _out_dependentobjects (`parent.GatherDependencies`))
  (return _out_dependentobjects))

(fn `GetLookAtDecription`
  (params (byCharacter :type "FGCharacterPlayer Object Reference") (state :type "UseState Structure (by ref)"))
  (returns (ReturnValue :type Text))
  (return (`parent.GetLookAtDecription` byCharacter state)))

(fn `IsUseable`
  (returns (ReturnValue :type Boolean))
  (bind _returnvalue (`parent.IsUseable`))
  (return _returnvalue))

(fn `NeedTransform`
  (returns (ReturnValue :type Boolean))
  (bind _returnvalue (`parent.NeedTransform`))
  (return _returnvalue))

(fn `PickUp`
  (params (inUser :type "FGCharacterPlayer Object Reference")))

(fn `ShouldSave`
  (returns (ReturnValue :type Boolean))
  (bind _returnvalue (`parent.ShouldSave`))
  (return _returnvalue))

(fn `UpdateUseState`
  (params (byCharacter :type "FGCharacterPlayer Object Reference") (atLocation :type "Vector Structure (by ref)") (componentHit :type "PrimitiveComponent Object Reference") (out_useState :type "UseState Structure (by ref)"))
  (`parent.UpdateUseState` byCharacter atLocation componentHit out_useState)
  (return))

(fn `UserConstructionScript`)