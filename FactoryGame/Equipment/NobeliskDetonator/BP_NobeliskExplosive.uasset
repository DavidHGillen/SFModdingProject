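; Blueprint for the Nobelisk explosive in the Nobelisk Detonator equipment set, serving as a thin child of its parent class.
; Explosion effects, hit handling and the save-related overrides (ShouldSave, GatherDependencies, NeedTransform) only forward to the parent.
; The multicast explosion-effects event, construction script and default lifecycle events are empty, so the graphs add no behavior of their own.
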(event `self.PlayExplosionEffects`
  (`parent.PlayExplosionEffects`))

(event `self.ReceiveHit`
  (params (MyComp :type "PrimitiveComponent Object Reference") (Other :type "Actor Object Reference") (OtherComp :type "PrimitiveComponent Object Reference") (bSelfMoved :type Boolean) (HitLocation :type "Vector Structure") (HitNormal :type "Vector Structure") (NormalImpulse :type "Vector Structure") (Hit :type "HitResult Structure (by ref)"))
  (`parent.ReceiveHit` MyComp Other OtherComp bSelfMoved HitLocation HitNormal NormalImpulse Hit))

(event `Multicast_PlayExplosionEffects`)

(fn `GatherDependencies`
  (returns (out_dependentObjects :type "Array of Object Object Reference"))
  (bind _out_dependentobjects (`parent.GatherDependencies`))
  (return _out_dependentobjects))

(fn `NeedTransform`
  (returns (ReturnValue :type Boolean))
  (bind _returnvalue (`parent.NeedTransform`))
  (return _returnvalue))

(fn `ShouldSave`
  (returns (ReturnValue :type Boolean))
  (bind _returnvalue (`parent.ShouldSave`))
  (return _returnvalue))

(fn `UserConstructionScript`)