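; BP_WAT1 is a prototype WAT actor whose graphs contain almost no logic of their own.
; Construction, significance gain and loss, and destruction only forward to the parent class.
; BeginPlay, overlap and Tick are disabled placeholders, and an OnLoaded callback does nothing.
; Functions named for alien SFX playback, a recently-rendered check and sending amplitude data to Niagara are empty stubs.
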(event `OnLoaded_B6148220483D04B067A000A9976DCD15`
  (params (Loaded :type "Object Object Reference")))

(event `FGSignificanceInterface.GainedSignificance`
  (`parent.GainedSignificance`))

(event `FGSignificanceInterface.LostSignificance`
  (`parent.LostSignificance`))

(event `self.ReceiveDestroyed`
  (`parent.ReceiveDestroyed`))

(fn `CheckIfRecentlyRendered`)

(fn `KillAlienSFX`)

(fn `PlayAlienSFX`)

(fn `SendAmplitudeDataToNiagara`)

(fn `UserConstructionScript`
  (`parent.UserConstructionScript`))