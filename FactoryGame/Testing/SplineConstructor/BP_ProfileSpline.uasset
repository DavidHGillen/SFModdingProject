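; Profile spline Blueprint in the testing SplineConstructor folder, apparently for profiling runs along a spline, with almost no logic of its own.
; Tick, StartProfile, construction and the current view and duration getters only forward to their parent versions.
; The player pawn, spawn-wait and debug-start events are empty, and the console variable, respawn and player controller functions return empty, false or invalid results.
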(event `self.ReceiveTick`
  (params (DeltaSeconds :type "Float (single-precision)"))
  (`parent.ReceiveTick` DeltaSeconds))

(event `self.StartProfile`
  (`parent.StartProfile`))

(event `FetchPlayerPawn`)

(event `EnsurePlayerDoneSpawning`)

(event `DebugStart`)

(fn `CheckDoneRespawning`
  (returns (bDoneSpawning :type Boolean))
  (return false))

(fn `GetConsoleVariableByName`
  (params (VariableName :type String))
  (returns (VariableInput :type String))
  (return ""))

(fn `GetCurrentDuration`
  (returns (ReturnValue :type "Float (double-precision)"))
  (bind _returnvalue (`parent.GetCurrentDuration`))
  (return _returnvalue))

(fn `GetCurrentView`
  (returns (ReturnValue :type "Transform Structure"))
  (bind _returnvalue (`parent.GetCurrentView`))
  (return _returnvalue))

(fn `GetPlayerController`
  (returns (bIsValid :type Boolean) (PlayerController :type "PlayerController Object Reference"))
  (return false null))

(fn `UserConstructionScript`
  (`parent.UserConstructionScript`))