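; BP_Planet is a sky environment planet Blueprint whose behavior comes almost entirely from its parent class.
; Preview, position, movement toggle and speed multiplier events only forward to parent implementations, while construction and material parameter updates are empty.
; Its save-game hooks are stubs, and it reports that it neither saves nor needs its transform stored.
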(event `FGSaveInterface.PreLoadGame`
  (params (saveVersion :type Integer) (gameVersion :type Integer)))

(event `self.UpdatePreview`
  (`parent.UpdatePreview`))

(event `FGSaveInterface.PreSaveGame`
  (params (saveVersion :type Integer) (gameVersion :type Integer)))

(event `self.SetPosition`
  (params (pct :type "Float (single-precision)"))
  (`parent.SetPosition` pct))

(event `self.EnableMovement`
  (params (enabled :type Boolean))
  (`parent.EnableMovement` enabled))

(event `self.SetMovementMultiplier`
  (params (multiplier :type "Float (single-precision)"))
  (`parent.SetMovementMultiplier` multiplier))

(event `FGSaveInterface.PostSaveGame`
  (params (saveVersion :type Integer) (gameVersion :type Integer)))

(event `FGSaveInterface.PostLoadGame`
  (params (saveVersion :type Integer) (gameVersion :type Integer)))

(fn `GatherDependencies`
  (returns (out_dependentObjects :type "Array of Object Object Reference"))
  (return))

(fn `NeedTransform`
  (returns (ReturnValue :type Boolean))
  (return false))

(fn `ShouldSave`
  (returns (ReturnValue :type Boolean))
  (return false))

(fn `UpdateMaterialParameters`)

(fn `UserConstructionScript`)