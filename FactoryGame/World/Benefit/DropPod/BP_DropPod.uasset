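; Drop pod Blueprint, a lootable world object that characters can look at, use and open.
; Its events for loot rolling, opening, look-at, use and repair only forward to the parent class, as do RequiresPowerToOpen and GetPowerConnection.
; Local power and repair functions are stubs: NeedsPower and NeedsRepair return false, power consumption is zero, and Repair does nothing.
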(event `self.ReceiveBeginPlay`
  (`parent.ReceiveBeginPlay`))

(event `self.RollLoot`
  (`parent.RollLoot`))

(event `self.OnOpened`
  (`parent.OnOpened`))

(event `FGUseableInterface.StopIsLookedAt`
  (params (byCharacter :type "FGCharacterPlayer Object Reference") (state :type "UseState Structure (by ref)"))
  (`parent.StopIsLookedAt` byCharacter state))

(event `FGUseableInterface.StartIsLookedAt`
  (params (byCharacter :type "FGCharacterPlayer Object Reference") (state :type "UseState Structure (by ref)"))
  (`parent.StartIsLookedAt` byCharacter state))

(event `FGUseableInterface.OnUse`
  (params (byCharacter :type "FGCharacterPlayer Object Reference") (state :type "UseState Structure (by ref)"))
  (`parent.OnUse` byCharacter state))

(event `self.OnRepair`
  (params (InteractingCharacter :type "FGCharacterPlayer Object Reference"))
  (`parent.OnRepair` InteractingCharacter))

(fn `GetPowerConnection`
  (returns (ReturnValue :type "FGPowerConnectionComponent Object Reference"))
  (bind _returnvalue (`parent.GetPowerConnection`))
  (return _returnvalue))

(fn `GetPowerConsumption`
  (returns (Power :type "Float (double-precision)"))
  (return 0.0))

(fn `GetRepairAmount`
  (returns (Amount :type "ItemAmount Structure"))
  (return))

(fn `NeedsPower`
  (returns (NeedsPower :type Boolean))
  (return false))

(fn `NeedsRepair`
  (returns (NeedsRepair :type Boolean))
  (return false))

(fn `Repair`
  (params (byCharacter :type "FGCharacterPlayer Object Reference")))

(fn `RequiresPowerToOpen`
  (returns (ReturnValue :type Boolean))
  (bind _returnvalue (`parent.RequiresPowerToOpen`))
  (return _returnvalue))

(fn `UserConstructionScript`)